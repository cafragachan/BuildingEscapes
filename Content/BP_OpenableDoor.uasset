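; BP_OpenableDoor is a door actor that swings open and closed in response to requests from its OpenDoor member.
; It stores its starting rotation at BeginPlay, then the DoorSwing timeline adds an animated yaw angle to it and rotates the whole actor.
; Open requests play the timeline and close requests reverse it, while a timeline event track plays the door lock sound at the actor's location.
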(event OnOpenRequest(OpenDoor)
  (bind _open_angle (Timeline|Door%20Swing Play)
    (:Update
      (Transformation|SetActorRotation (Math|Rotator|CombineRotators (Variables|Default|GetInitial%20Rotation) (Math|Rotator|MakeRotator 0.0 0.0 _open_angle))))
    (:Sound
      (Audio|PlaySoundatLocation "/Game/Audio/door-lock.door-lock" (Transformation|GetActorLocation)))))

(event OnCloseRequest(OpenDoor)
  (bind _open_angle (Timeline|Door%20Swing Reverse)
    (:Update
      (Transformation|SetActorRotation (Math|Rotator|CombineRotators (Variables|Default|GetInitial%20Rotation) (Math|Rotator|MakeRotator 0.0 0.0 _open_angle))))
    (:Sound
      (Audio|PlaySoundatLocation "/Game/Audio/door-lock.door-lock" (Transformation|GetActorLocation)))))

(event EventBeginPlay
  (Variables|Default|SetInitial%20Rotation (Transformation|GetActorRotation)))

(fn ConstructionScript)